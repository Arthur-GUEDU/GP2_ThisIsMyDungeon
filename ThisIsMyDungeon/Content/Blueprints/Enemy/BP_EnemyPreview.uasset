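; Enemy preview character that repeatedly travels from its start location to the level objective between waves, with a Niagara effect active along the way.
; It spawns its own controller, takes the objective from BP_LevelDefinitionActor and uses AI MoveTo, teleporting back on success to loop.
; Enemy manager subsystem events hide and deactivate it on wave start, then reset and restart it on wave end.
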(event Custom|GoToObjective
  (bind _niagara (Variables|Default|GetNiagara))
  (bind _niagara_2 (Variables|Default|GetNiagara))
  (AI|AIMoveTo (Class|PawnMovementComponent|GetPawnOwner (Variables|Character|GetCharacterMovement)) (Variables|Default|GetObjective) 0 5.0 false
    (:OnSuccess
      (Development|SetHiddeninGame _niagara true false)
      (Components|Activation|Deactivate _niagara)
      (Transformation|SetActorLocation (Variables|Default|GetStartPos) false false)
      (Development|SetHiddeninGame _niagara_2 false false)
      (Components|Activation|Activate _niagara_2 true)
      (CallFunction|GotoObjective))))

(event Custom|Activate
  (bind _niagara (Variables|Default|GetNiagara))
  (Transformation|SetActorLocation (Variables|Default|GetStartPos) false false)
  (Components|Activation|Activate (Variables|Character|GetCharacterMovement) false)
  (Components|Activation|Activate (Variables|Character|GetMesh) false)
  (Components|Activation|SetActive (Variables|Collision|GetCapsuleComponent) true false)
  (Rendering|SetActorHiddenInGame false)
  (Development|SetHiddeninGame _niagara false false)
  (Components|Activation|Activate _niagara true))

(event Custom|WaveStart
  (CallFunction|Deactivate))

(event Custom|Deactivate
  (bind _niagara (Variables|Default|GetNiagara))
  (Components|Activation|Deactivate (Variables|Character|GetCharacterMovement))
  (Components|Activation|Deactivate (Variables|Character|GetMesh))
  (Components|Activation|SetActive (Variables|Collision|GetCapsuleComponent) false false)
  (Rendering|SetActorHiddenInGame true)
  (Development|SetHiddeninGame _niagara true false)
  (Components|Activation|Deactivate _niagara))

(event Custom|WaveEnd
  (CallFunction|Activate)
  (CallFunction|GotoObjective))

(event EventBeginPlay
  (bind _returnvalue (Subsystems|GetEnemyManagerInstanceSubsystem))
  (bind _niagara (Variables|Default|GetNiagara))
  (Pawn|SpawnDefaultController)
  (Variables|Default|SetStartPos (Transformation|GetActorLocation))
  (bind _returnvalue_2 (Actor|GetActorOfClass "/Game/Levels/BP_LevelDefinitionActor.BP_LevelDefinitionActor_C"))
  (Variables|Default|SetObjective (Transformation|GetActorLocation (Variables|/Script/TPS_ThisIsMyDungeon.LevelDefinitionActor|GetObjectiveActor _returnvalue_2)))
  (EventDispatchers|AssignOnWaveStart _returnvalue (delegate Custom|WaveStart))
  (EventDispatchers|BindEventtoOnWaveEnd _returnvalue (delegate Custom|WaveEnd))
  (CallFunction|GotoObjective)
  (Development|SetHiddeninGame _niagara false false)
  (Components|Activation|Activate _niagara true))

(event Collision|EventActorBeginOverlap
  (params (OtherActor :type Actor%20Object%20Reference)))

(event EventTick
  (params (DeltaSeconds :type Float%20%28single-precision%29)))

(fn ConstructionScript)