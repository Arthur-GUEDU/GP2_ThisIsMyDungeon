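; BP_PlayerProjectile is the player's projectile Blueprint, handling its sound and visual feedback.
; BeginPlay binds handlers to the projectile's fired, hit and destroyed events.
; Firing plays a pitch-randomized 2D shot sound and starts a random flight sound on the Audio component, with a rare secret variant.
; Hits play a 2D impact sound, and destruction spawns a feather Niagara effect at the projectile's location.
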(event Custom|ProjectileDestroyed
  ;[1 1 1] Destroy Logic FX / SFX
  (Niagara|SpawnSystematLocation "/Game/VFX/NS_Feather.NS_Feather" (Transformation|GetActorLocation)))

(event Custom|ProjectileFired
  (bind _audio (Variables|Default|GetAudio))
  ;[1 1 1] Projectile Fired Event
  (Audio|PlaySound2D (Variables|Default|GetFireSoundCue) 0.5 (Math|Random|RandomFloatinRange 0.8 1.4) 0.0 0 self false)
  (if (> (Math|Random|RandomFloat) 0.95)
    (Audio|Components|Audio|SetSound _audio (Variables|Default|GetSecretFlySoundsCue))
    (else
      (Audio|Components|Audio|SetSound _audio (.OutItem (Utilities|Array|Random (Variables|Default|GetFlySoundsCues))))))
  (Audio|Components|Audio|Play _audio 0.0))

(event Custom|Projectile%20Hit%20Event
  ;[1 1 1] Projectile Hit
  (Audio|PlaySound2D (Variables|Default|GetHitSoundCue) 1.0 1.0 0.0 0 self false))

(event EventBeginPlay
  (EventDispatchers|BindEventtoOnProjectileDestroyed (delegate Custom|ProjectileDestroyed))
  (EventDispatchers|BindEventtoOnProjectileFired (delegate Custom|ProjectileFired))
  (EventDispatchers|BindEventtoOnProjectileHit (delegate Custom|Projectile%20Hit%20Event)))

(fn ConstructionScript)