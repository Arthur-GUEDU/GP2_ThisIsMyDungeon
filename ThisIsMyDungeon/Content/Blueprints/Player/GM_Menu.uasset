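; Menu game mode that plays looping-style background music and drives camera transitions between main, level selection and credits screens.
; Stores three level cameras, then each transition switches the view target and plays a level sequence, reversed when returning to main.
; Each transition binds a callback to the sequence's finish.
; Separate handlers update the menu HUD widgets to show, hide or focus the matching screen.
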(event EventBeginPlay
  (bind _returnvalue (Audio|CreateSound2D "/Game/SFX/Drunken_Sailor_Cue.Drunken_Sailor_Cue" 1.0 1.0 0.0 0))
  (bind _output_get (Variables|Default|SetMainMenuMusic _returnvalue))
  (Audio|Components|Audio|Play _output_get 0.0))

(event EventTick
  (params (DeltaSeconds :type Float%20%28single-precision%29)))

(fn ConstructionScript)

(fn SetLevelCameras
  (params (Cameras :type Array%20of%20Camera%20Actor%20Object%20References))
  (Variables|Default|SetMainCamera (Utilities|Array|Get(acopy) Cameras))
  (Variables|Default|SetLevelsCamera (Utilities|Array|Get(acopy) Cameras 1))
  (Variables|Default|SetCreditsCamera (Utilities|Array|Get(acopy) Cameras 2)))

(fn MaintoLevelSequence
  (bind _sequenceplayer (CallFunction|PlaySequence "/Game/Sequences/LevelSelectionMenu.LevelSelectionMenu" (Variables|Default|GetMainCamera) false))
  (EventDispatchers|BindEventtoOnFinished _sequenceplayer (EventDispatchers|CreateEvent :!event OnLevelMenu)))

(fn MaintoCreditsSequence
  (bind _sequenceplayer (CallFunction|PlaySequence "/Game/Sequences/CreditsMenu.CreditsMenu" (Variables|Default|GetCreditsCamera) false))
  (EventDispatchers|BindEventtoOnFinished _sequenceplayer (EventDispatchers|CreateEvent :!event OnCreditsMenu)))

(fn LeveltoMainSequence
  (bind _sequenceplayer (CallFunction|PlaySequence "/Game/Sequences/LevelSelectionMenu.LevelSelectionMenu" (Variables|Default|GetLevelsCamera) true))
  (EventDispatchers|BindEventtoOnFinished _sequenceplayer (EventDispatchers|CreateEvent :!event OnMainMenu)))

(fn CreditstoMainSequence
  (bind _sequenceplayer (CallFunction|PlaySequence "/Game/Sequences/CreditsMenu.CreditsMenu" (Variables|Default|GetCreditsCamera) true))
  (EventDispatchers|BindEventtoOnFinished _sequenceplayer (EventDispatchers|CreateEvent :!event OnMainMenu)))

(fn OnCreditsMenu
  (bind _asbp_menu_hud (Utilities|Casting|CastToBP_MenuHUD (HUD|GetHUD (Game|GetPlayerController 0))))
  (Default|ShowCreditsMenu (Variables|/Game/Blueprints/UserInterface/Menu/BP_MenuHUD.BP_MenuHUD_C|GetMainMenu _asbp_menu_hud)))

(fn OnMainMenu
  (bind _asbp_menu_hud (Utilities|Casting|CastToBP_MenuHUD (HUD|GetHUD (Game|GetPlayerController 0))))
  (Default|ShowMainMenu (Variables|/Game/Blueprints/UserInterface/Menu/BP_MenuHUD.BP_MenuHUD_C|GetMainMenu _asbp_menu_hud))
  (Game|Player|SetViewTargetwithBlend (Game|GetPlayerController 0) (Variables|Default|GetMainCamera) 0.0 "VTBlend_Linear" 0.0 false))

(fn OnLevelMenu
  (bind _asbp_menu_hud (Utilities|Casting|CastToBP_MenuHUD (HUD|GetHUD (Game|GetPlayerController 0))))
  (Default|HideMenu (Variables|/Game/Blueprints/UserInterface/Menu/BP_MenuHUD.BP_MenuHUD_C|GetMainMenu _asbp_menu_hud))
  (Default|FocusLevelMenu (Variables|/Game/Blueprints/UserInterface/Menu/BP_MenuHUD.BP_MenuHUD_C|GetLevelMenu _asbp_menu_hud)))

(fn PlaySequence
  (params (LevelSequence :type Level%20Sequence%20Object%20Reference) (CameraTarget :type Actor%20Object%20Reference) (bPlayReversed :type Boolean))
  (Game|Player|SetViewTargetwithBlend (Game|GetPlayerController 0) CameraTarget 0.0 "VTBlend_Linear" 0.0 false)
  (bind _outactor (Sequencer|Player|CreateLevelSequencePlayer LevelSequence))
  (if bPlayReversed
    (Class|MovieSceneSequencePlayer|PlayReverse (Variables|/Script/LevelSequence.LevelSequenceActor|GetSequencePlayer _outactor))
    (else
      (Sequencer|Player|Play (Variables|/Script/LevelSequence.LevelSequenceActor|GetSequencePlayer _outactor) :!class /Script/MovieScene.MovieSceneSequencePlayer)))
  (return (Variables|/Script/LevelSequence.LevelSequenceActor|GetSequencePlayer _outactor)))