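; BP_Player is the pirate captain player character, with a parrot projectile and a trap edit mode.
; BeginPlay spawns the trap editor and a reusable projectile, creates the HUD, and binds hit and death feedback.
; Projectile events toggle parrot visibility and start the cooldown.
; Input events drive pause and trap UI, alongside respawn, trap-placement montages and debug spawn/damage keys.
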(event Custom|Pause/Resume
  (bind _returnvalue (Game|GetPlayerController 0))
  ;[1 1 1] Pause Menu
  (if (Variables|Default|GetbIsPaused)
    (Variables|Default|SetbIsPaused false)
    (Default|HidePauseMenu (Variables|/Game/Blueprints/UserInterface/Game/BP_HUD.BP_HUD_C|GetPauseUI (stale _asbp_hud)))
    (Input|SetInputModeGameOnly _returnvalue false)
    (Variables|/Script/Engine.PlayerController|SetbShowMouseCursor _returnvalue false)
    (Game|SetGamePaused false)
    (else
      (Variables|Default|SetbIsPaused true)
      (bind _asbp_hud (Utilities|Casting|CastToBP_HUD (HUD|GetHUD _returnvalue)))
      (UserInterface|Viewport|AddtoViewport (Variables|/Game/Blueprints/UserInterface/Game/BP_HUD.BP_HUD_C|GetPauseUI _asbp_hud) 0)
      (Input|SetInputModeGameandUI _returnvalue (Variables|/Game/Blueprints/UserInterface/Buttons/WB_MenuButton.WB_MenuButton_C|GetCustomButton (Variables|/Game/Blueprints/UserInterface/Game/WB_PauseMenu.WB_PauseMenu_C|GetWB_ResumeButton (Variables|/Game/Blueprints/UserInterface/Game/BP_HUD.BP_HUD_C|GetPauseUI _asbp_hud))) "DoNotLock" true false)
      (Default|ShowPauseMenu (Variables|/Game/Blueprints/UserInterface/Game/BP_HUD.BP_HUD_C|GetPauseUI _asbp_hud))
      (Variables|/Script/Engine.PlayerController|SetbShowMouseCursor _returnvalue true)
      (Game|SetGamePaused true))))

(event Custom|OnProjectileFired_Event
  ;[1 1 1] Projectiles events
  (Rendering|SetVisibility (Variables|Default|GetParrot) false false))

(event Custom|OnPlayerHit_Event
  ;[1 1 1] Player Hit Logic + FX / SFX
  (if (not (Variables|Default|GetbIsDead))
    (Animation|PlayAnimMontage "/Game/Assets/Animations/Player/Characters_Captain_Barbarossa_HitAnimation_Montage.Characters_Captain_Barbarossa_HitAnimation_Montage" 0.8 "None")
    (Audio|PlaySound2D "/Game/SFX/SC_Pirate_Hit.SC_Pirate_Hit" 1.0 1.0 0.0 0 0)))

(event Custom|OnPlayerDeath_Event
  (bind _playerhud (Variables|Default|GetPlayerHUD))
  (bind _playerdeathui (Variables|/Game/Blueprints/UserInterface/Game/BP_HUD.BP_HUD_C|GetPlayerDeathUI _playerhud))
  ;[1 1 1] Player Death Logic + FX / SFX
  (UserInterface|Viewport|AddtoViewport _playerdeathui 0)
  (Default|StartDeathUIAnim _playerdeathui)
  (bind _asplayer_controller (Utilities|Casting|CastToPlayerController (Pawn|GetController)))
  (Input|DisableInput _asplayer_controller)
  (Audio|PlaySound2D "/Game/SFX/SC_Pirate_Death.SC_Pirate_Death" 1.0 1.0 0.0 0 0))

(event Custom|Respawn
  ;[1 1 1] Respawn
  (Class|PlayerCharacter|RespawnPlayer)
  (bind _asplayer_controller (Utilities|Casting|CastToPlayerController (Pawn|GetController)))
  (Input|EnableInput _asplayer_controller))

(event Custom|ProjectileDestroyed
  ;[1 1 1] Projectiles events
  (Rendering|SetVisibility (Variables|Default|GetParrot) true false)
  (Class|Timer|SetupTimerandStart (Variables|Default|GetProjectileCDTimer) (Variables|Default|GetProjectileCDTime) (Variables|Default|GetProjectileCDTimeStamp)))

(event Input|EnhancedActionEvents|EnhancedInputActionIA_Pause
  (params (ActionValue :type Boolean) (ElapsedSeconds :type Float%20%28double-precision%29) (TriggeredSeconds :type Float%20%28double-precision%29) (InputAction :type Input%20Action%20Object%20Reference :default "/Game/Inputs/IA_Pause.IA_Pause"))
  (bind _returnvalue (Game|GetPlayerController 0))
  ;[1 1 1] Pause Menu
  (:Started
    (if (Variables|Default|GetbIsPaused)
      (Variables|Default|SetbIsPaused false)
      (Default|HidePauseMenu (Variables|/Game/Blueprints/UserInterface/Game/BP_HUD.BP_HUD_C|GetPauseUI (stale _asbp_hud)))
      (Input|SetInputModeGameOnly _returnvalue false)
      (Variables|/Script/Engine.PlayerController|SetbShowMouseCursor _returnvalue false)
      (Game|SetGamePaused false)
      (else
        (Variables|Default|SetbIsPaused true)
        (bind _asbp_hud (Utilities|Casting|CastToBP_HUD (HUD|GetHUD _returnvalue)))
        (UserInterface|Viewport|AddtoViewport (Variables|/Game/Blueprints/UserInterface/Game/BP_HUD.BP_HUD_C|GetPauseUI _asbp_hud) 0)
        (Input|SetInputModeGameandUI _returnvalue (Variables|/Game/Blueprints/UserInterface/Buttons/WB_MenuButton.WB_MenuButton_C|GetCustomButton (Variables|/Game/Blueprints/UserInterface/Game/WB_PauseMenu.WB_PauseMenu_C|GetWB_ResumeButton (Variables|/Game/Blueprints/UserInterface/Game/BP_HUD.BP_HUD_C|GetPauseUI _asbp_hud))) "DoNotLock" true false)
        (Default|ShowPauseMenu (Variables|/Game/Blueprints/UserInterface/Game/BP_HUD.BP_HUD_C|GetPauseUI _asbp_hud))
        (Variables|/Script/Engine.PlayerController|SetbShowMouseCursor _returnvalue true)
        (Game|SetGamePaused true)))))

(event Input|EnhancedActionEvents|EnhancedInputActionIA_SwitchMode
  (params (ActionValue :type Boolean) (ElapsedSeconds :type Float%20%28double-precision%29) (TriggeredSeconds :type Float%20%28double-precision%29) (InputAction :type Input%20Action%20Object%20Reference :default "/Game/Inputs/IA_SwitchMode.IA_SwitchMode"))
  ;[1 1 1] Edit mode UI
  (Default|ChangeModeUI (Variables|/Game/Blueprints/UserInterface/Game/BP_HUD.BP_HUD_C|GetPlayerUI (Variables|Default|GetPlayerHUD)) (Variables|Default|GetbIsEditMode)))

(event Input|EnhancedActionEvents|EnhancedInputActionIA_TrapUINav
  (params (ActionValue :type Float%20%28double-precision%29) (ElapsedSeconds :type Float%20%28double-precision%29) (TriggeredSeconds :type Float%20%28double-precision%29) (InputAction :type Input%20Action%20Object%20Reference :default "/Game/Inputs/IA_TrapUINav.IA_TrapUINav"))
  ;[1 1 1] Edit mode UI
  (if (Variables|Default|GetbIsEditMode)
    (Default|ChangeTrapUI (Variables|/Game/Blueprints/UserInterface/Game/BP_HUD.BP_HUD_C|GetPlayerUI (Variables|Default|GetPlayerHUD)) (Variables|Default|GetCurrentTrapIndex))))

(event EventBeginPlay
  ;[1 1 1] Begin Play
  (bind _returnvalue (Game|SpawnActorfromClass "/Game/Blueprints/Traps/BP_TrapEdition.BP_TrapEdition_C" (Math|Transform|MakeTransform "0, 0, 0" "0, 0, 0" "1.000000,1.000000,1.000000") "Undefined" "MultiplyWithRoot" 0 0))
  (Variables|Default|SetTrapEdition _returnvalue)
  (EventDispatchers|AssignOnPlayerHit (delegate Custom|OnPlayerHit_Event))
  (EventDispatchers|BindEventtoOnPlayerDeath (delegate Custom|OnPlayerDeath_Event))
  (bind _returnvalue_2 (Game|SpawnActorfromClass "/Game/Blueprints/Player/BP_PlayerProjectile.BP_PlayerProjectile_C" (Math|Transform|MakeTransform "0.000000,0.000000,-100.000000" "0, 0, 0" "1.000000,1.000000,1.000000") "Undefined" "MultiplyWithRoot" 0 0))
  (bind _output_get (Variables|Default|SetProjectile _returnvalue_2))
  (EventDispatchers|BindEventtoOnProjectileDestroyed _output_get (delegate Custom|ProjectileDestroyed))
  (EventDispatchers|AssignOnProjectileFired _output_get (delegate Custom|OnProjectileFired_Event))
  (bind _asbp_hud (Utilities|Casting|CastToBP_HUD (HUD|GetHUD (Game|GetPlayerController 0))))
  (bind _output_get_2 (Variables|Default|SetPlayerHUD _asbp_hud))
  (Default|CreateHUD _output_get_2))

(event EventOnTrapPlaced
  (params (IsTrapPlaced :type Boolean))
  (if IsTrapPlaced
    (Animation|PlayAnimMontage "/Game/Assets/Animations/Player/Characters_Captain_Barbarossa_YesAnimation_Montage.Characters_Captain_Barbarossa_YesAnimation_Montage" 1.0 "None")
    (else
      (Animation|PlayAnimMontage "/Game/Assets/Animations/Player/Characters_Captain_Barbarossa_NoAnimation_Montage.Characters_Captain_Barbarossa_NoAnimation_Montage" 1.0 "None"))))

(event Input|KeyboardEvents|DebugKeyM
  (params (Key :type Key%20Structure :default "None") (ActionValue :type Input%20Action%20Value%20Structure))
  ;[0.8049 1 0] Debug
  (:Pressed
    (Game|Damage|ApplyDamage self 1e+01 0 0)))

(event Input|KeyboardEvents|DebugKeyU
  (params (Key :type Key%20Structure :default "None") (ActionValue :type Input%20Action%20Value%20Structure))
  ;[0.8049 1 0] Debug
  (:Pressed
    (Class|EnemyManagerInstanceSubsystem|Spawn (Subsystems|GetEnemyManagerInstanceSubsystem))))

(fn ConstructionScript)