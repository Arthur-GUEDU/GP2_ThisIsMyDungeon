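; GM_Player is the game mode Blueprint that handles the win and loss end states of a level.
; On BeginPlay it binds loss to the death of the level definition's objective actor and victory to the EnemyManager subsystem's level-end event.
; Each outcome shows its BP_HUD widget, focuses a menu or retry button and pauses the game.
; The mouse cursor is shown on victory but hidden on loss.
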(event Custom|OnGameLoose
  (bind _returnvalue (Game|GetPlayerController 0))
  ;[1 1 1] On player loose behavior
  (bind _asbp_hud (Utilities|Casting|CastToBP_HUD (HUD|GetHUD _returnvalue)))
  (UserInterface|Viewport|AddtoViewport (Variables|/Game/Blueprints/UserInterface/Game/BP_HUD.BP_HUD_C|GetLooseUI _asbp_hud) 0)
  (Input|SetInputModeGameandUI _returnvalue (Variables|/Game/Blueprints/UserInterface/Buttons/WB_LevelButton.WB_LevelButton_C|GetCustomButton (Variables|/Game/Blueprints/UserInterface/Game/WB_LooseUI.WB_LooseUI_C|GetWB_RetryButton (Variables|/Game/Blueprints/UserInterface/Game/BP_HUD.BP_HUD_C|GetLooseUI _asbp_hud))) "DoNotLock" false false)
  (Variables|/Script/Engine.PlayerController|SetbShowMouseCursor _returnvalue false)
  (Default|ShowLooseUI (Variables|/Game/Blueprints/UserInterface/Game/BP_HUD.BP_HUD_C|GetLooseUI _asbp_hud))
  (Game|SetGamePaused true))

(event Custom|OngameWin
  (bind _returnvalue (Game|GetPlayerController 0))
  ;[1 1 1] On player win behavior
  (bind _asbp_hud (Utilities|Casting|CastToBP_HUD (HUD|GetHUD _returnvalue)))
  (UserInterface|Viewport|AddtoViewport (Variables|/Game/Blueprints/UserInterface/Game/BP_HUD.BP_HUD_C|GetWinUI _asbp_hud) 0)
  (Input|SetInputModeGameandUI _returnvalue (Variables|/Game/Blueprints/UserInterface/Buttons/WB_MenuButton.WB_MenuButton_C|GetCustomButton (Variables|/Game/Blueprints/UserInterface/Game/WB_WinUI.WB_WinUI_C|GetWB_MenuButton (Variables|/Game/Blueprints/UserInterface/Game/BP_HUD.BP_HUD_C|GetWinUI _asbp_hud))) "DoNotLock" false false)
  (Variables|/Script/Engine.PlayerController|SetbShowMouseCursor _returnvalue true)
  (Default|ShowVictoryMenu (Variables|/Game/Blueprints/UserInterface/Game/BP_HUD.BP_HUD_C|GetWinUI _asbp_hud))
  (Game|SetGamePaused true))

(event EventBeginPlay
  (bind _returnvalue (Subsystems|GetEnemyManagerInstanceSubsystem))
  (EventDispatchers|AssignOnObjectiveDeath (Variables|/Script/TPS_ThisIsMyDungeon.LevelDefinitionActor|GetObjectiveActor (Class|EnemyManagerInstanceSubsystem|GetLevelDef _returnvalue)) (delegate Custom|OnGameLoose))
  (EventDispatchers|BindEventtoOnLevelEnd _returnvalue (delegate Custom|OngameWin)))

(fn ConstructionScript)